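; Map info point actor that shows an icon or a text panel as the player enters its trigger volumes.
; IconTrigger toggles the icon widget, while InfoTrigger swaps it for a Map_Info widget filled with header and info text on BeginPlay.
; While the player is inside InfoTrigger, a Gate and one-frame Delay loop keeps the info panel rotated toward the Player_BP camera.
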(event `self.ReceiveBeginPlay`
  (`SceneComponent.SetVisibility` (`self.Widget`) false false)
  (bind _asmap_info (cast `/Game/Core/Tests/Map_Info` (`WidgetComponent.GetWidget` (`self.Widget`))))
  (`/Game/Core/Tests/Map_Info.Update Text` _asmap_info (`self.Header Text`) (`self.Info Text`))
  (bind _returnvalue (`GameplayStatics.GetActorOfClass` "/Game/Core/Player/BluePrints/Player_BP.Player_BP_C")))

(event `self.Info Trigger.OnComponentBeginOverlap`
  (params (OverlappedComponent :type "PrimitiveComponent Object Reference") (OtherActor :type "Actor Object Reference") (OtherComp :type "PrimitiveComponent Object Reference") (OtherBodyIndex :type Integer) (bFromSweep :type Boolean) (SweepResult :type "HitResult Structure (by ref)"))
  (bind _returnvalue (`GameplayStatics.GetWorldDeltaSeconds`))
  (bind _widget (`self.Widget`))
  (cast `/Game/Core/Player/BluePrints/Player_BP` OtherActor)
  (`SceneComponent.SetVisibility` (`self.Widget`) true false)
  (`SceneComponent.SetVisibility` (`self.Widget1`) false false)
  (`|ExecutionSequence`
    (:`then_0`
      (goto _label_2 :!via `Open`))
    (:`then_1`
      (`KismetSystemLibrary.Delay` _returnvalue)
      (`SceneComponent.K2_SetWorldRotation` _widget (`KismetMathLibrary.FindLookAtRotation` (`SceneComponent.K2_GetComponentLocation` _widget) (`SceneComponent.K2_GetComponentLocation` (`/Game/Core/Player/BluePrints/Player_BP.Camera` (stale `self.ReceiveBeginPlay` _returnvalue)))) false false :!label _label)
      (`/Engine/EditorBlueprintResources/StandardMacros.Gate` false :!label _label_2
        (:`Exit`
          (`KismetSystemLibrary.Delay` _returnvalue)
          (goto _label))))))

(event `self.Info Trigger.OnComponentEndOverlap`
  (params (OverlappedComponent :type "PrimitiveComponent Object Reference") (OtherActor :type "Actor Object Reference") (OtherComp :type "PrimitiveComponent Object Reference") (OtherBodyIndex :type Integer))
  (cast `/Game/Core/Player/BluePrints/Player_BP` OtherActor)
  (`SceneComponent.SetVisibility` (`self.Widget`) false false)
  (`SceneComponent.SetVisibility` (`self.Widget1`) true false)
  (goto _label_2 :!via `Close`))

(event `self.Icon Trigger.OnComponentBeginOverlap`
  (params (OverlappedComponent :type "PrimitiveComponent Object Reference") (OtherActor :type "Actor Object Reference") (OtherComp :type "PrimitiveComponent Object Reference") (OtherBodyIndex :type Integer) (bFromSweep :type Boolean) (SweepResult :type "HitResult Structure (by ref)"))
  (cast `/Game/Core/Player/BluePrints/Player_BP` OtherActor)
  (`SceneComponent.SetVisibility` (`self.Widget1`) true false))

(event `self.Icon Trigger.OnComponentEndOverlap`
  (params (OverlappedComponent :type "PrimitiveComponent Object Reference") (OtherActor :type "Actor Object Reference") (OtherComp :type "PrimitiveComponent Object Reference") (OtherBodyIndex :type Integer))
  (cast `/Game/Core/Player/BluePrints/Player_BP` OtherActor)
  (`SceneComponent.SetVisibility` (`self.Widget1`) false false))

(fn `UserConstructionScript`)