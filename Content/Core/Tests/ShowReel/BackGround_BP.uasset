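; BackGround_BP is a show reel room actor that takes hold of the player when they overlap its box.
; Entry enables input, reveals the room meshes, lights and exit, hides the background, optionally plays audio, and fires once until reset.
; An open gate then pins Player_BP to the Arrow's X/Y every tick, keeping its Z.
; Pressing E reverses this, moves the player to ExitSocket and re-arms the trigger.
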(event `self.ReceiveBeginPlay`
  (bind _returnvalue (`GameplayStatics.GetActorOfClass` "/Game/Core/Player/BluePrints/Player_BP.Player_BP_C")))

(event `self.ReceiveTick`
  (params (DeltaSeconds :type "Float (single-precision)"))
  (bind (_returnvalue_x _returnvalue_y) (`KismetMathLibrary.BreakVector` (`SceneComponent.K2_GetComponentLocation` (`self.Arrow`))))
  (`/Engine/EditorBlueprintResources/StandardMacros.Gate` true :!label _label
    (:`Exit`
      (bind (_returnvalue_x_2 _returnvalue_y_2 _returnvalue_z) (`KismetMathLibrary.BreakVector` (`self.K2_GetActorLocation` (stale `self.ReceiveBeginPlay` _returnvalue))))
      (`self.K2_SetActorLocation` (stale `self.ReceiveBeginPlay` _returnvalue) (`KismetMathLibrary.MakeVector` _returnvalue_x _returnvalue_y _returnvalue_z) false false))))

(event `self.Box.OnComponentBeginOverlap`
  (params (OverlappedComponent :type "PrimitiveComponent Object Reference") (OtherActor :type "Actor Object Reference") (OtherComp :type "PrimitiveComponent Object Reference") (OtherBodyIndex :type Integer) (bFromSweep :type Boolean) (SweepResult :type "HitResult Structure (by ref)"))
  (`self.EnableInput` (`GameplayStatics.GetPlayerController` 0))
  (`/Engine/EditorBlueprintResources/StandardMacros.DoOnce` false :!label _label_2
    (:`Completed`
      (set `self.In ShowRoom?` true)
      (`SceneComponent.SetVisibility` (`self.StaticMesh`) true true)
      (`SceneComponent.SetVisibility` (`self.RectLight1`) true true)
      (`SceneComponent.SetVisibility` (`self.RectLight2`) true true)
      (`SceneComponent.SetVisibility` (`self.Box`) true true)
      (`SceneComponent.SetVisibility` (`self.EXIT`) true true)
      (`SceneComponent.SetVisibility` (`self.RectLight`) true true)
      (if (`self.Use Music?`)
        (`AudioComponent.Play` (`self.Audio`) 0.0))
      (`SceneComponent.SetVisibility` (`self.BackGround`) false false)
      (goto _label :!via `Open`))))

(event `Key|E`
  (params (Key :type "Key Structure"))
  (:`Pressed`
    (`self.DisableInput` (`GameplayStatics.GetPlayerController` 0))
    (`AudioComponent.Stop` (`self.Audio`))
    (`SceneComponent.SetVisibility` (`self.StaticMesh`) false false)
    (`SceneComponent.SetVisibility` (`self.RectLight1`) false false)
    (`SceneComponent.SetVisibility` (`self.RectLight2`) false false)
    (`SceneComponent.SetVisibility` (`self.Box`) false false)
    (`SceneComponent.SetVisibility` (`self.EXIT`) false false)
    (`SceneComponent.SetVisibility` (`self.RectLight`) false false)
    (`SceneComponent.SetVisibility` (`self.BackGround`) true false)
    (set `self.In ShowRoom?` false)
    (`self.K2_SetActorLocation` (stale `self.ReceiveBeginPlay` _returnvalue) (`SceneComponent.K2_GetComponentLocation` (`self.Exit Socket`)) false false)
    (`|ExecutionSequence`
      (:`then_0`
        (goto _label :!via `Close`))
      (:`then_1`
        (goto _label_2 :!via `Reset`)))))

(fn `UserConstructionScript`)