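; Shooting range target: a dummy that takes bullet damage, falls when its life runs out, then resets, optionally sliding along a trail.
; It binds to the weapon's bullet hit event, scales damage by proximity to the head box, and reports kills to the range widget.
; A timeline animates the knockdown, while Tick eases the base back and forth between trail sockets, driving trail audio from velocity.
; The construction script sizes the trail and positions the base.
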(event `self.ReceiveBeginPlay`
  (bind _returnvalue (`GameplayStatics.GetActorOfClass` "/Game/Core/Player/BluePrints/Player_BP.Player_BP_C"))
  (set `self.Player BP` _returnvalue)
  (bind _returnvalue_2 (`GameplayStatics.GetActorOfClass` "/Game/Core/Weapons/BluePrints/Universal_Weapons.Universal_Weapons_C"))
  (bind _output_get (set `self.Universal Weapon` _returnvalue_2))
  (add `/Game/Core/Weapons/BluePrints/Universal_Weapons.Bullet Hit Event` _output_get (`|CreateDelegate` :!event `Bullet Hit`)))

(event `Bullet Hit`
  (params (`Out Hit` :type "HitResult Structure") (`Hit Delay` :type "Float (double-precision)") (Damage :type Integer))
  (bind (_bblockinghit _binitialoverlap _time _distance _location _impactpoint _normal _impactnormal _physmat _hitactor _hitcomponent) (`GameplayStatics.BreakHitResult` `Out Hit`))
  (if (== _hitcomponent (`self.Dummy`))
    (if (<= (`self.Dummy Life`) 0.0)
      (`/Engine/EditorBlueprintResources/StandardMacros.DoOnce` false :!label _label
        (:`Completed`
          (`GameplayStatics.PlaySound2D` "/Game/Core/NPC/Enemys/Sound/Kill/SW_Kill_Enemy.SW_Kill_Enemy" 0.5 1.0 0.0 null null)
          (`GameplayStatics.SpawnSoundAtLocation` "/Game/Core/Map/MultiPlayer/Shoot_Range/BluePrints/Sound/SW_Shooting_Range_Target_Down.SW_Shooting_Range_Target_Down" (`self.K2_GetActorLocation`) (struct) 1.0 1.0 0.0 "/Game/Core/Common/Sound/Physical_Materials/Foot_Sounds/Custom_SoundAttenuation.Custom_SoundAttenuation" null)
          (bind _foundwidgets (`WidgetBlueprintLibrary.GetAllWidgetsOfClass` "/Game/Core/Map/MultiPlayer/Shoot_Range/UI/Shootig_Range.Shootig_Range_C" false))
          (`/Game/Core/Map/MultiPlayer/Shoot_Range/UI/Shootig_Range.Add Target Hit` (`|GetArrayItem` _foundwidgets))
          (bind (_direction _newtrack_0) (`Timeline|Timeline` :!via `PlayFromStart`)
            (:`Update`
              (`SceneComponent.K2_SetRelativeRotation` (`self.Dummy`) (`KismetMathLibrary.MakeRotator` 0.0 _newtrack_0) false false))
            (:`Finished`
              (set `self.Dummy Life` 150.0)
              (goto _label :!via `Reset`))
            (:`NewTrack_1`
              (`GameplayStatics.SpawnSoundAtLocation` "/Game/Core/Map/MultiPlayer/Shoot_Range/BluePrints/Sound/SW_Shooting_Range_Target_Reposition.SW_Shooting_Range_Target_Reposition" (`self.K2_GetActorLocation`) (struct) 1.0 1.0 0.0 "/Game/Core/Common/Sound/Physical_Materials/Foot_Sounds/Custom_SoundAttenuation.Custom_SoundAttenuation" null)))))
      (else
        (set `self.Dummy Life` (- (`self.Dummy Life`) (`KismetMathLibrary.FClamp` (- (* Damage 2.5) (/ (`KismetMathLibrary.Vector_Distance` _location (`SceneComponent.K2_GetComponentLocation` (`self.Head Box`))) 2.0)) (- Damage 10) 100000.0)))
        (if (<= (`self.Dummy Life`) 0.0)
          (goto _label))))))

(event `self.ReceiveTick`
  (params (DeltaSeconds :type "Float (single-precision)"))
  (bind _trail_sfx (`self.Trail SFX`))
  (bind _trail (`self.Trail`))
  (bind _alpha (`self.Alpha`))
  (bind _alpha_2 (`self.Alpha`))
  (bind _returnvalue (/ 0.34 (`self.Trail Length`)))
  (if (`self.Use Trail Moviment`)
    (`|ExecutionSequence`
      (:`then_0`
        (`AudioComponent.SetVolumeMultiplier` _trail_sfx (`KismetMathLibrary.FInterpTo` (`AudioComponent.VolumeMultiplier` _trail_sfx) (`self.SFX Target`) 0.1 1.0))
        (`AudioComponent.SetPitchMultiplier` _trail_sfx (`KismetMathLibrary.FInterpTo` (`AudioComponent.PitchMultiplier` _trail_sfx) (+ 1.0 (`KismetMathLibrary.FClamp` (/ (stale _velocity) 100.0))) 0.1 1.0))
        (set `self.Alpha` (`KismetMathLibrary.FInterpTo` (`self.Alpha`) (`self.Target`) 0.1 (/ (`self.Moviment Duration`) (`KismetMathLibrary.FClamp` (/ (`self.Trail Length`) 2.0) 0.1 100000.0))))
        (`SceneComponent.K2_SetWorldLocation` (`self.Base`) (`KismetMathLibrary.VLerp` (`SceneComponent.GetSocketLocation` _trail "Start") (`SceneComponent.GetSocketLocation` _trail "End") (`KismetMathLibrary.Lerp` (+ _alpha _returnvalue) (- _alpha _returnvalue) _alpha)) false false)
        (`/Engine/EditorBlueprintResources/StandardMacros.DoOnce` false :!label _label_2
          (:`Completed`
            (`/Engine/EditorBlueprintResources/StandardMacros.FlipFlop`
              (:`A`
                (set `self.Target` 1.0))
              (:`B`
                (set `self.Target` 0.0)))
            (`KismetSystemLibrary.Delay` (+ (`self.Moviment Delay to Return`) (`KismetMathLibrary.Abs` (`KismetMathLibrary.RandomFloat`))))
            (goto _label_2 :!via `Reset`))))
      (:`then_1`
        (bind _velocity (`/Game/Core/Weapons/BluePrints/Exential/MacroLibrary.Get Velocity` (`self.Base`)))
        (set `self.SFX Target` (`KismetMathLibrary.FClamp` (/ _velocity 100.0)))))
    (elif (!= _alpha_2 0.0)
      (set `self.Alpha` (`KismetMathLibrary.FInterpTo` _alpha_2 0.0 0.1 1.0)))))

(fn `UserConstructionScript`
  (bind _trail (`self.Trail`))
  (bind _alpha (`self.Alpha`))
  (bind _trail_length (`self.Trail Length`))
  (bind _returnvalue (/ 0.34 _trail_length))
  (`SceneComponent.SetRelativeScale3D` (`self.Trail`) (`KismetMathLibrary.MakeVector` 1.0 _trail_length 1.0))
  (`SceneComponent.K2_SetWorldLocation` (`self.Base`) (`KismetMathLibrary.VLerp` (`SceneComponent.GetSocketLocation` _trail "Start") (`SceneComponent.GetSocketLocation` _trail "End") (`KismetMathLibrary.Lerp` (+ _alpha _returnvalue) (- _alpha _returnvalue) _alpha)) false false))