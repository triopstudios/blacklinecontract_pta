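; Sound_Box is a speaker prop that plays music, animates to it and reacts to being shot.
; The construction script assigns the track, and Tick drives the woofer mesh's Bass and Pitch morph targets from the music's cooked envelope data.
; BeginPlay binds to the bullet hit event of a single Universal_Weapons actor found by class.
; A hit on the box turns on physics for its support mesh and randomly stops the music.
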(event `self.ReceiveBeginPlay`
  (bind _returnvalue (`GameplayStatics.GetActorOfClass` "/Game/Core/Weapons/BluePrints/Universal_Weapons.Universal_Weapons_C"))
  (add `/Game/Core/Weapons/BluePrints/Universal_Weapons.Bullet Hit Event` _returnvalue (delegate `CustomEvent`)))

(event `self.ReceiveTick`
  (params (DeltaSeconds :type "Float (single-precision)"))
  (bind _sound_woofers (`self.sound_woofers`))
  (bind _outenvelopedata (`AudioComponent.GetCookedEnvelopeData` (`self.Music`)))
  (`SkeletalMeshComponent.SetMorphTarget` _sound_woofers "Bass" _outenvelopedata false)
  (`SkeletalMeshComponent.SetMorphTarget` _sound_woofers "Pitch" _outenvelopedata false))

(event `CustomEvent`
  (params (`Out Hit` :type "HitResult Structure") (`Hit Delay` :type "Float (double-precision)") (Damage :type Integer))
  (if (== (`.HitActor` (`GameplayStatics.BreakHitResult` `Out Hit`)) self)
    (`PrimitiveComponent.SetSimulatePhysics` (`self.sound_box_support`) true)
    (if (`KismetMathLibrary.RandomBool`)
      (`AudioComponent.Stop` (`self.Music`)))))

(fn `UserConstructionScript`
  (`AudioComponent.SetSound` (`self.Music`) (`self.New Sound`)))