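; Target cannon that fires physics discs as shootable targets, in a test multiplayer map folder.
; A hold interaction, with an optional button, clears old discs and starts a timed series of spawned static mesh discs launched by randomized impulses.
; Weapon bullet-hit events destroy struck discs with sound and debris effects.
; Chained vector spring interpolation on Tick wobbles the pitch and yaw pivots after brief kicks from launches and hits.
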(event `self.ReceiveBeginPlay`
  ;[0 0 0 1 30] Target Cannon
  (bind _returnvalue (`GameplayStatics.GetActorOfClass` "/Game/Core/Weapons/BluePrints/Universal_Weapons.Universal_Weapons_C"))
  (bind _output_get (set `self.NewVar` _returnvalue))
  (add `/Game/Core/Weapons/BluePrints/Universal_Weapons.Bullet Hit Event` _output_get (`|CreateDelegate` :!event `Event Hit - Disc`))
  (bind _returnvalue_2 (`GameplayStatics.GetActorOfClass` "/Game/Core/Player/BluePrints/Player_BP.Player_BP_C"))
  (add `/Game/Core/Player/BluePrints/Player_BP.Hit Interactive EXC` _returnvalue_2 (`|CreateDelegate` :!event `CustomEvent`))
  (`self.EnableInput` (`GameplayStatics.GetPlayerController` 0)))

(event `Start Launch`
  (bind _box (`self.Box`))
  (bind _disc_count (`self.Disc Count`))
  (bind _newvar_0 (`self.NewVar_0`))
  (bind _disc_active (`self.Disc Active`))
  (bind _disc (`self.Disc`))
  (bind (_returnvalue_location _returnvalue_rotation) (`KismetMathLibrary.BreakTransform` (`SceneComponent.GetRelativeTransform` _box)))
  (bind _returnvalue (or (== _disc_count 1) (== _disc_count 2)))
  ;[0 0 0 1 30] Target Cannon
  (`self.NewMacro` (struct :`Pitch` 0.5 :`Yaw` 0.5))
  (set `self.Is Launching?` true)
  (if (not (`KismetArrayLibrary.Array_IsEmpty` _disc_active))
    (for _array_element _disc_active
      (`/Engine/EditorBlueprintResources/StandardMacros.IsValid` _array_element
        (:`Is Valid`
          (`ActorComponent.K2_DestroyComponent` _array_element)))))
  (`KismetArrayLibrary.Array_Clear` (`self.Disc Active`))
  (`GameplayStatics.PlaySoundAtLocation` "/Game/Core/Map/MultiPlayer/Only_For_Test/Blueprints/Targets/Disc_Launcher/Sounds/SW_Disc_Launch_Start.SW_Disc_Launch_Start" (`self.K2_GetActorLocation`) (struct) 1.0 1.0 0.0 "/Game/Core/Common/Sound/Physical_Materials/Foot_Sounds/Custom_SoundAttenuation.Custom_SoundAttenuation" null null null)
  (`KismetSystemLibrary.Delay` 1.31)
  (if (== (`KismetMathLibrary.SelectInt` _newvar_0 (- _newvar_0 1) _returnvalue) (`KismetMathLibrary.SelectInt` _disc_count (- _disc_count 1) _returnvalue)) :!label _label
    (set `self.NewVar_0` 0)
    (set `self.Is Launching?` false)
    (else
      (bind _returnvalue_2 (`AddComponent|NODE_AddStaticMeshComponent-1` :`bManualAttachment` true :`RelativeTransform` (`KismetMathLibrary.MakeTransform` _returnvalue_location _returnvalue_rotation (0.25 0.25 0.015224))))
      (bind _output_get (set `self.Disc` _returnvalue_2))
      (`KismetArrayLibrary.Array_Add` (`self.Disc Active`) _output_get)
      (`SceneComponent.K2_AttachToComponent` _returnvalue_2 _box "None" "SnapToTarget" "SnapToTarget" "KeepWorld" true)
      (`|ExecutionSequence`
        (:`then_0`
          (set `self.Target` (struct :`Pitch` 5.0))
          (`/Engine/EditorBlueprintResources/StandardMacros.IncrementInt` (`self.NewVar_0`)
            (:`  `
              (`GameplayStatics.PlaySoundAtLocation` "/Game/Core/Map/MultiPlayer/Only_For_Test/Blueprints/Targets/Disc_Launcher/Sounds/SW_Disc_Launch.SW_Disc_Launch" (`self.K2_GetActorLocation`) (struct) 1.0 (`KismetMathLibrary.RandomFloatInRange` 0.95 1.05) 0.0 "/Game/Core/Common/Sound/Physical_Materials/Foot_Sounds/Custom_SoundAttenuation.Custom_SoundAttenuation" null null null)
              (`PrimitiveComponent.SetCollisionResponseToAllChannels` _disc "ECR_Block")
              (`PrimitiveComponent.SetSimulatePhysics` _disc true)
              (`PrimitiveComponent.AddImpulse` _disc (* (`SceneComponent.GetForwardVector` (`self.Launch Pitch`)) 100000 (`KismetMathLibrary.SelectFloat` 0.9 1.1 (`KismetMathLibrary.RandomBool`))) "None" false)
              (`KismetSystemLibrary.Delay` (`self.Launch Time`))
              (goto _label))))
        (:`then_1`
          (`KismetSystemLibrary.Delay` 0.1)
          (set `self.Target` (struct)))))))

(event `Event Hit - Disc`
  (params (`Out Hit` :type "HitResult Structure") (`Hit Delay` :type "Float (double-precision)") (Damage :type Integer))
  (bind (_bblockinghit _binitialoverlap _time _distance _location _impactpoint _normal _impactnormal _physmat _hitactor _hitcomponent) (`GameplayStatics.BreakHitResult` `Out Hit`))
  ;[0 0 0 1 30] Target Cannon
  (if (== _hitcomponent (`self.Launch Pitch`))
    (`self.NewMacro` (struct :`Pitch` 5.0)))
  (for (_array_element _array_index) (`self.Disc Active`)
    (if (== _hitcomponent _array_element)
      (bind _returnvalue (`SceneComponent.K2_GetComponentLocation` _array_element))
      (`GameplayStatics.SpawnSoundAtLocation` "/Game/Core/Map/MultiPlayer/Only_For_Test/Blueprints/Targets/Disc_Launcher/Sounds/Hit/Hit_Disc_Target.Hit_Disc_Target" _returnvalue (struct) 1.5 1.0 0.0 null null)
      (`NiagaraFunctionLibrary.SpawnSystemAtLocation` "/Game/Core/Niagara_VFX/Niagara/Destruction/Destruction_Concrete.Destruction_Concrete" _returnvalue)
      (`ActorComponent.K2_DestroyComponent` _array_element)
      (`KismetArrayLibrary.Array_Remove` (`self.Disc Active`) _array_index))))

(event `self.ReceiveTick`
  (params (DeltaSeconds :type "Float (single-precision)"))
  (bind (_target_roll _target_pitch _target_yaw) (`KismetMathLibrary.BreakRotator` (`self.Target`)))
  (bind (_rotation_roll _rotation_pitch _rotation_yaw) (`KismetMathLibrary.BreakRotator` (`self.Rotation`)))
  (bind (_rotation_roll_2 _rotation_pitch_2 _rotation_yaw_2) (`KismetMathLibrary.BreakRotator` (`self.Rotation`)))
  (bind (_relativerotation_roll _relativerotation_pitch _relativerotation_yaw) (`KismetMathLibrary.BreakRotator` (`SceneComponent.RelativeRotation` (`self.Launch Yaw`))))
  (bind (_relativerotation_roll_2 _relativerotation_pitch_2) (`KismetMathLibrary.BreakRotator` (`SceneComponent.RelativeRotation` (`self.Launch Pitch`))))
  ;[0 0 0 1 30] Target Cannon
  (bind _returnvalue (`KismetMathLibrary.VectorSpringInterp` (`KismetMathLibrary.MakeVector` 0.0 (+ _relativerotation_pitch_2 _target_pitch) (+ _relativerotation_yaw _target_yaw)) (`KismetMathLibrary.MakeVector` _rotation_roll_2 _rotation_pitch_2 _rotation_yaw_2) (make `VectorSpringState`) 1.0 0.2 0.1 0.25))
  (bind (_returnvalue_x _returnvalue_y _returnvalue_z) (`KismetMathLibrary.BreakVector` (* _returnvalue -1)))
  (bind _returnvalue_2 (`KismetMathLibrary.VectorSpringInterp` _returnvalue (`KismetMathLibrary.MakeVector` 0.0 _returnvalue_y (+ _returnvalue_z _returnvalue_y)) (make `VectorSpringState`) 0.5 0.2 0.1 0.25))
  (bind _returnvalue_3 (`KismetMathLibrary.VectorSpringInterp` _returnvalue_2 (* (`KismetMathLibrary.MakeVector` _rotation_roll _rotation_pitch _rotation_yaw) 1.8) (make `VectorSpringState`) 1.0 0.2 0.1 0.25))
  (`SceneComponent.K2_SetRelativeRotation` (`self.Launch Pitch`) (`KismetMathLibrary.MakeRotator` 0.0 (.y _returnvalue_3)) false false)
  (`SceneComponent.K2_SetRelativeRotation` (`self.Launch Yaw`) (`KismetMathLibrary.MakeRotator` 0.0 0.0 (.z _returnvalue_3)) false false))

(event `InputAction|Interact Actor` :consume false :overrideparent false
  (params (Key :type "Key Structure"))
  ;[0 0 0 1 30] Target Cannon
  (:`Pressed`
    (if (and (== (`.HitActor` (`GameplayStatics.BreakHitResult` (stale `CustomEvent` `Hit Result`))) self) (not (`self.Is Launching?`)))
      (`/Game/Core/Weapons/BluePrints/Exential/MacroLibrary.Interaction Hold` 0.5 :!label _label_2
        (:`Interact`
          (`self.Start Launch`)))))
  (:`Released`
    (goto _label_2 :!via `Close`)))

(event `CustomEvent`
  (params (`Hit Result` :type "HitResult Structure") (`Player BP` :type "/Game/Core/Player/BluePrints/Player_BP Object Reference"))
  (bind (_bblockinghit _binitialoverlap _time _distance _location _impactpoint _normal _impactnormal _physmat _hitactor _hitcomponent) (`GameplayStatics.BreakHitResult` `Hit Result`))
  (bind _returnvalue (`KismetSystemLibrary.IsValid` (`self.Sphere1`)))
  (bind _returnvalue_2 (== _hitcomponent (`self.Sphere1`)))
  ;[0 0 0 1 30] Target Cannon
  (if (== _hitactor self)
    (`/Game/Core/Weapons/BluePrints/Exential/MacroLibrary.Interaction UI` `Player BP` self "NewEnumerator4" (`KismetMathLibrary.SelectString` "Wait Finish" "Enable Disc Launcher" (`self.Is Launching?`)) 0 false (select `bool` _returnvalue :`false` true :`true` (not _returnvalue_2)) (select `bool` _returnvalue :`true` _returnvalue_2) (`SceneComponent.K2_GetComponentLocation` (select `bool` _returnvalue :`false` (`self.DefaultSceneRoot`) :`true` (`self.Button`) :!type "SceneComponent Object Reference")) true)))

(fn `UserConstructionScript`
  (bind (_rotation_roll _rotation_pitch _rotation_yaw) (`KismetMathLibrary.BreakRotator` (`self.Rotation`)))
  (`SceneComponent.K2_SetRelativeRotation` (`self.Launch Pitch`) (`KismetMathLibrary.MakeRotator` 0.0 _rotation_pitch) false false)
  (`SceneComponent.K2_SetRelativeRotation` (`self.Launch Yaw`) (`KismetMathLibrary.MakeRotator` 0.0 0.0 _rotation_yaw) false false)
  (if (not (`self.Use Button?`))
    (`ActorComponent.K2_DestroyComponent` (`self.Button`))
    (`ActorComponent.K2_DestroyComponent` (`self.Sphere1`))
    (`ActorComponent.K2_DestroyComponent` (`self.Sphere`))))