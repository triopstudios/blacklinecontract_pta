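; Interactive elevator for the zombie mode that carries between a start and end point when the player interacts with it.
; A FlipFlop alternates playing and reversing a Timeline that lerps the platform and two sliding doors, with a DoOnce blocking re-triggering mid-ride.
; It flags OnElevator on ZMBGlobalBP while moving.
; If TeleportZombies is set, arrival destroys all zombies after a delay and respawns them through CustomSpawn, alternating spawn sets.
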(event `self.ReceiveBeginPlay`
  (bind _returnvalue (`GameplayStatics.GetActorOfClass` "/Game/Core/Player/BluePrints/Player_BP.Player_BP_C"))
  (`self.EnableInput` (`GameplayStatics.GetPlayerController` 0))
  (bind _returnvalue_2 (`GameplayStatics.GetActorOfClass` "/Game/Core/NPC/Zombies/ZMB-Global-BP.ZMB-Global-BP_C"))
  (set `self.ZMB Global` _returnvalue_2)
  (`SceneComponent.K2_SetWorldLocation` (`self.Elevator`) (`SceneComponent.K2_GetComponentLocation` (`self.Start`)) false false))

(event `InputAction|Interact Actor` :consume false
  (params (Key :type "Key Structure"))
  (:`Pressed`
    (if (== (`.HitActor` (`GameplayStatics.BreakHitResult` (`/Game/Core/Player/BluePrints/Player_BP.Hit Interactive` (stale `self.ReceiveBeginPlay` _returnvalue)))) self)
      (`/Engine/EditorBlueprintResources/StandardMacros.DoOnce` false :!label _label
        (:`Completed`
          (`GameplayStatics.PlaySound2D` "/Game/Core/NPC/Zombies/Elevator/Music/SW_Elevator_Moving.SW_Elevator_Moving" 1.0 1.0 0.0 null null)
          (`/Engine/EditorBlueprintResources/StandardMacros.FlipFlop`
            (:`A`
              (bind (_direction _newtrack_0 _newtrack_1) (`Timeline|Timeline` :!via `PlayFromStart` :!label _label_2)
                (:`Update`
                  (`SceneComponent.K2_SetWorldLocation` (`self.Elevator`) (`KismetMathLibrary.VLerp` (`SceneComponent.K2_GetComponentLocation` (`self.Start`)) (`SceneComponent.K2_GetComponentLocation` (`self.End`)) _newtrack_0) false false)
                  (`SceneComponent.K2_SetRelativeLocation` (`self.Elevator_Door`) (`KismetMathLibrary.VLerp` (200.0 0.0 0.0) (0.0 0.0 0.0) _newtrack_1) false false)
                  (`SceneComponent.K2_SetRelativeLocation` (`self.Elevator_Door2`) (`KismetMathLibrary.VLerp` (-200.0 0.0 0.0) (0.0 0.0 0.0) _newtrack_1) false false)
                  (set `/Game/Core/NPC/Zombies/ZMB-Global-BP.On elevator?` true (`self.ZMB Global`)))
                (:`Finished`
                  (`|ExecutionSequence`
                    (:`then_0`
                      (if (`self.Teleport Zombies`)
                        (`KismetArrayLibrary.Array_Clear` (`self.Zombie Array`))
                        (bind _isa (`/Engine/EditorBlueprintResources/StandardMacros.FlipFlop`)
                          (:`A`
                            _)
                          (:`B`
                            _))
                        (bind _outactors (`GameplayStatics.GetAllActorsOfClass` "/Game/Core/NPC/Zombies/Zombie_NPC.Zombie_NPC_C"))
                        (for _array_element _outactors
                          (`KismetArrayLibrary.Array_Add` (`self.Zombie Array`) _array_element))
                        (`KismetSystemLibrary.Delay` 3.0)
                        (for _array_element_2 (`self.Zombie Array`)
                          (`self.K2_DestroyActor` _array_element_2))
                        (`/Game/Core/NPC/Zombies/ZMB-Global-BP.Custom Spawn` (`self.ZMB Global`) (select `bool` _isa :`false` (`self.Spawns Default Location`) :`true` (`self.Spawns New Location`)) (- (`KismetArrayLibrary.Array_Length` (`self.Zombie Array`)) 1))))
                    (:`then_1`
                      (set `/Game/Core/NPC/Zombies/ZMB-Global-BP.On elevator?` false (`self.ZMB Global`))
                      (goto _label :!via `Reset`))))))
            (:`B`
              (goto _label_2 :!via `ReverseFromEnd`))))))))

(fn `UserConstructionScript`
  (`SceneComponent.K2_SetWorldLocation` (`self.Elevator`) (`SceneComponent.K2_GetComponentLocation` (`self.Start`)) false false))