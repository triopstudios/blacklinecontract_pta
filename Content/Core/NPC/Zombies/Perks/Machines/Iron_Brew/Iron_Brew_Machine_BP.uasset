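; Iron-Brew perk machine for Zombies that sells the player a one-time max health increase.
; It shows a buy prompt through the player's interact hit event and purchases on a held interact input, checking points only when zombie mode is active.
; A purchase charges via ZMBGlobalBP, holsters the weapon, spawns a perk bottle on the player, raises max life, adds a HUD icon and plays the jingle.
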(event `self.ReceiveBeginPlay`
  (bind _returnvalue (`GameplayStatics.GetActorOfClass` "/Game/Core/Player/BluePrints/Player_BP.Player_BP_C"))
  (set `self.Player BP` _returnvalue)
  (add `/Game/Core/Player/BluePrints/Player_BP.Hit Interactive EXC` (`self.Player BP`) (delegate `Interact`))
  (bind _returnvalue_2 (`GameplayStatics.GetActorOfClass` "/Game/Core/NPC/Zombies/ZMB-Global-BP.ZMB-Global-BP_C"))
  (set `self.ZMB Global` _returnvalue_2)
  (bind _returnvalue_3 (`GameplayStatics.GetActorOfClass` "/Game/Core/Weapons/BluePrints/Universal_Weapons.Universal_Weapons_C"))
  (set `self.UVW BP` _returnvalue_3)
  (`self.EnableInput` (`GameplayStatics.GetPlayerController` 0)))

(event `Interact`
  (params (`Hit Result` :type "HitResult Structure") (`Player BP` :type "/Game/Core/Player/BluePrints/Player_BP Object Reference"))
  (`/Game/Core/Weapons/BluePrints/Exential/MacroLibrary.Interaction UI` `Player BP` self "NewEnumerator1" "Iron-Brew" (`self.Value $`) (`/Game/Core/NPC/Zombies/ZMB-Global-BP.Zombie Mode Active?` (`self.ZMB Global`)) false true (`SceneComponent.K2_GetComponentLocation` (`self.Box`))))

(event `InputAction|Interact Actor` :consume false
  (params (Key :type "Key Structure"))
  (bind _music (`self.Music`))
  (bind _uvw_bp (`self.UVW BP`))
  (bind _weapon_holster_anim (`/Game/Core/Weapons/BluePrints/Universal_Weapons.Weapon Holster Anim` _uvw_bp))
  (bind _player (`/Game/Core/Player/BluePrints/Player_BP.Player` (`self.Player BP`)))
  (:`Pressed`
    (if (== (`.HitActor` (`GameplayStatics.BreakHitResult` (stale `Interact` `Hit Result`))) self)
      (`/Game/Core/Weapons/BluePrints/Exential/MacroLibrary.Interaction Hold` 0.5 :!label _label
        (:`Interact`
          (if (`/Game/Core/NPC/Zombies/ZMB-Global-BP.Zombie Mode Active?` (`self.ZMB Global`))
            (if (>= (`/Game/Core/NPC/Zombies/ZMB-Global-BP.Points Number` (`self.ZMB Global`)) (`self.Value $`))
              (`/Engine/EditorBlueprintResources/StandardMacros.DoOnce` false :!label _label_2
                (:`Completed`
                  (`GameplayStatics.PlaySound2D` "/Game/Core/NPC/Zombies/Common_Sounds/Shop___/Sounds/SW_Buy_Accept.SW_Buy_Accept" 1.0 1.0 0.0 null null)
                  (`self.DisableInput` (`self.UVW BP`) (`GameplayStatics.GetPlayerController` 0))
                  (`/Game/Core/NPC/Zombies/ZMB-Global-BP.On Buy` (`self.ZMB Global`) (`self.Value $`))
                  (set `/Game/Core/Player/BluePrints/Player_BP.Global Anim` true (`self.Player BP`))
                  (`/Game/Core/Weapons/BluePrints/Universal_Weapons.Holster For Interact` _uvw_bp)
                  (`KismetSystemLibrary.Delay` (- (`AnimSequenceBase.SequenceLength` _weapon_holster_anim) (`AnimMontage.GetDefaultBlendOutTime` _weapon_holster_anim)))
                  (bind _returnvalue (`|SpawnActorFromClass` "/Game/Core/NPC/Zombies/Perks/Perk_Bottle/Perk_Bottle_BP.Perk_Bottle_BP_C" (`SceneComponent.K2_GetComponentToWorld` _player) "AlwaysSpawn" "MultiplyWithRoot" null "/Game/Core/NPC/Zombies/Perks/Perk_Bottle/Texture/Iron-Brew/MI_Perk_Bottle_Iron-Brew.MI_Perk_Bottle_Iron-Brew" null))
                  (`self.K2_AttachToComponent` _returnvalue _player "None" "KeepWorld" "KeepWorld" "KeepWorld" true)
                  (set `/Game/Core/Player/BluePrints/Player_BP.Player Life Max` 250 (`self.Player BP`))
                  (bind _returnvalue_2 (`|GenericCreateObject` "/Game/Core/NPC/Zombies/Zombie_HUD/Perks-PowerUp_Icons.Perks-PowerUp_Icons_C" "/Game/Core/NPC/Zombies/Zombie_HUD/Icons/Perks/T_Iron-Brew_Icon.T_Iron-Brew_Icon"))
                  (`PanelWidget.AddChild` (`/Game/Core/NPC/Zombies/Zombie_HUD/Zombie_Mode.Perks` (`/Game/Core/NPC/Zombies/ZMB-Global-BP.Hud` (`self.ZMB Global`))) _returnvalue_2)
                  (`AudioComponent.SetSound` _music "/Game/Core/NPC/Zombies/Perks/Machines/Iron_Brew/Music/SW_Iron_Brew_End.SW_Iron_Brew_End")
                  (`AudioComponent.Play` _music 0.0)
                  (`AudioComponent.SetVolumeMultiplier` _music 1.0)))
              (else
                (`GameplayStatics.PlaySound2D` "/Game/Core/NPC/Zombies/Common_Sounds/Shop___/Sounds/SW_Buy_no_Points.SW_Buy_no_Points" 1.0 1.0 0.0 null null)))
            (else
              (goto _label_2)))))))
  (:`Released`
    (goto _label :!via `Close`)))

(fn `UserConstructionScript`)