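; Perk bottle actor for the Zombies perk system that plays the perk-use animation on the player and itself, then removes itself.
; On BeginPlay it applies the perk material to the liquid, switches the player mesh to Animation Blueprint mode and starts both montages together.
; When the player montage blends out or is interrupted, it redraws the weapon, re-enables its input, clears the player's GlobalAnim flag and destroys itself.
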(event `self.ReceiveBeginPlay`
  (`PrimitiveComponent.SetMaterial` (`self.Perk_liquid`) 0 (`self.Perk Material`))
  (bind _returnvalue (`GameplayStatics.GetActorOfClass` "/Game/Core/Player/BluePrints/Player_BP.Player_BP_C"))
  (bind _player (`/Game/Core/Player/BluePrints/Player_BP.Player` _returnvalue))
  (`SkeletalMeshComponent.SetAnimationMode` _player "AnimationBlueprint" true)
  (`|PlayMontage` _player "/Game/Core/NPC/Zombies/Perks/Perk_Bottle/Anims/Player_Perk_anim_Montage.Player_Perk_anim_Montage"
    (:`then`
      (`|PlayMontage` (`self.SkeletalMesh1`) "/Game/Core/NPC/Zombies/Perks/Perk_Bottle/Anims/Perk_anim_use_Montage.Perk_anim_use_Montage"))
    (:`OnBlendOut`
      (bind _returnvalue_2 (`GameplayStatics.GetActorOfClass` "/Game/Core/Weapons/BluePrints/Universal_Weapons.Universal_Weapons_C" :!label _label))
      (`/Game/Core/Weapons/BluePrints/Universal_Weapons.Draw For Interact` _returnvalue_2)
      (`self.EnableInput` _returnvalue_2 (`GameplayStatics.GetPlayerController` 0))
      (set `/Game/Core/Player/BluePrints/Player_BP.Global Anim` false _returnvalue)
      (`self.K2_DestroyActor`))
    (:`OnInterrupted`
      (goto _label))))

(fn `UserConstructionScript`)