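; Zombie mystery box that shows a random weapon pickup, charging points through ZMBGlobalBP when zombie mode is active.
; A short interact hold while the player targets it starts a once-guarded open montage with sound and lights.
; A timeline then repeatedly swaps a child actor among random weapon classes, disabling collision and flagging each as MysteryBox.
; The pickup hides after a timeout, while a delay loop polls the child actor to trigger the montage's closing section.
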(event `self.ReceiveBeginPlay`
  (`self.EnableInput` (`GameplayStatics.GetPlayerController` 0))
  (bind _returnvalue (`GameplayStatics.GetActorOfClass` "/Game/Core/NPC/Zombies/ZMB-Global-BP.ZMB-Global-BP_C"))
  (set `self.ZMB_BP` _returnvalue)
  (bind _returnvalue_2 (`GameplayStatics.GetActorOfClass` "/Game/Core/Player/BluePrints/Player_BP.Player_BP_C"))
  (add `/Game/Core/Player/BluePrints/Player_BP.Hit Interactive EXC` _returnvalue_2 (`|CreateDelegate` :!event `Interact`)))

(event `InputAction|Interact Actor` :consume false
  (params (Key :type "Key Structure"))
  (bind _zmb_bp (`self.ZMB_BP`))
  (bind _weapons_pickup (`self.Weapons Pickup`))
  (bind _aspickup_weapon_base (cast `/Game/Core/Weapons/Pickup_Weapons/Pickup_weapon_Base` (`ChildActorComponent.ChildActor` (`self.Weapon PickUp`)) :!pure true))
  (:`Pressed`
    (if (== (`.HitActor` (`GameplayStatics.BreakHitResult` (`/Game/Core/Player/BluePrints/Player_BP.Hit Interactive` (stale `self.ReceiveBeginPlay` _returnvalue_2)))) self)
      (`/Game/Core/Weapons/BluePrints/Exential/MacroLibrary.Interaction Hold` 0.25 :!label _label
        (:`Interact`
          (if (`/Game/Core/NPC/Zombies/ZMB-Global-BP.Zombie Mode Active?` _zmb_bp)
            (if (>= (`/Game/Core/NPC/Zombies/ZMB-Global-BP.Points Number` _zmb_bp) (`self.Value $$`))
              (`/Engine/EditorBlueprintResources/StandardMacros.DoOnce` false :!label _label_2
                (:`Completed`
                  (`/Engine/EditorBlueprintResources/StandardMacros.IsValid` (`self.ZMB_BP`)
                    (:`Is Valid`
                      (`/Game/Core/NPC/Zombies/ZMB-Global-BP.On Buy` (`self.ZMB_BP`) (`self.Value $$`)))
                    (:`Is Not Valid`
                      _))
                  (`GameplayStatics.PlaySound2D` "/Game/Core/NPC/Zombies/Common_Sounds/Shop___/Sounds/SW_Buy_Accept.SW_Buy_Accept" 1.0 1.0 0.0 null null)
                  (`|PlayMontage` (`self.Safe_Box-Rig`) "/Game/Core/NPC/Zombies/Mystery-Box/Animations/Safe_Box-Rig_Open_Montage.Safe_Box-Rig_Open_Montage"
                    (:`then`
                      (`GameplayStatics.PlaySoundAtLocation` "/Game/Core/NPC/Zombies/Mystery-Box/Sound/SW_mysterybox-Open_1.SW_mysterybox-Open_1" (`self.K2_GetActorLocation`) (struct) 1.0 1.01 0.0 "/Game/Core/Common/Sound/Physical_Materials/Foot_Sounds/Custom_SoundAttenuation.Custom_SoundAttenuation" null null null)
                      (`SceneComponent.SetVisibility` (`self.PointLight`) true false)
                      (`SceneComponent.SetVisibility` (`self.PointLight1`) true false)
                      (`KismetSystemLibrary.Delay` 3.3)
                      (`SceneComponent.SetVisibility` (`self.Weapon PickUp`) true false)
                      (bind (_direction _newtrack_0) (`Timeline|Timeline` :!via `PlayFromStart`)
                        (:`Update`
                          (`KismetSystemLibrary.Delay` (- _newtrack_0 (`GameplayStatics.GetWorldDeltaSeconds`)))
                          (`ChildActorComponent.SetChildActorClass` (`self.Weapon PickUp`) (`|GetArrayItem` _weapons_pickup (`KismetMathLibrary.RandomIntegerInRange` 0 (- (`KismetArrayLibrary.Array_Length` _weapons_pickup) 1))))
                          (`self.SetActorEnableCollision` _aspickup_weapon_base false)
                          (set `/Game/Core/Weapons/Pickup_Weapons/Pickup_weapon_Base.Mystery Box?` true _aspickup_weapon_base)
                          (`KismetSystemLibrary.RetriggerableDelay` 0.3)
                          (set `/Game/Core/Weapons/Pickup_Weapons/Pickup_weapon_Base.Mystery Box?` true _aspickup_weapon_base)
                          (`self.SetActorEnableCollision` _aspickup_weapon_base false))
                        (:`Finished`
                          (`KismetSystemLibrary.Delay` 7.5)
                          (`SceneComponent.SetVisibility` (`self.Weapon PickUp`) false false))
                        (:`NewTrack_1`
                          (if (== (`ChildActorComponent.ChildActor` (`self.Weapon PickUp`)) null) :!label _label_3
                            (`/Engine/EditorBlueprintResources/StandardMacros.DoOnce` false :!label _label_4
                              (:`Completed`
                                (`|PlayMontage` (`self.Safe_Box-Rig`) "/Game/Core/NPC/Zombies/Mystery-Box/Animations/Safe_Box-Rig_Open_Montage.Safe_Box-Rig_Open_Montage" 1.0 15.0
                                  (:`OnCompleted`
                                    (`SceneComponent.SetVisibility` (`self.PointLight`) false false)
                                    (`SceneComponent.SetVisibility` (`self.PointLight1`) false false)
                                    (goto _label_4 :!via `Reset`)))))
                            (else
                              (`KismetSystemLibrary.Delay` 0.2)
                              (goto _label_3))))))
                    (:`OnCompleted`
                      (`SceneComponent.SetVisibility` (`self.PointLight`) false false)
                      (`SceneComponent.SetVisibility` (`self.PointLight1`) false false)
                      (goto _label_2 :!via `Reset`))
                    (:`OnInterrupted`
                      (goto _label_2 :!via `Reset`)))))
              (else
                (`GameplayStatics.PlaySound2D` "/Game/Core/NPC/Zombies/Common_Sounds/Shop___/Sounds/SW_Buy_no_Points.SW_Buy_no_Points" 1.0 1.0 0.0 null null)))
            (else
              (goto _label_2)))))))
  (:`Released`
    (goto _label :!via `Close`)))

(event `Interact`
  (params (`Hit Result` :type "HitResult Structure") (`Player BP` :type "/Game/Core/Player/BluePrints/Player_BP Object Reference"))
  (`/Game/Core/Weapons/BluePrints/Exential/MacroLibrary.Interaction UI` `Player BP` self "NewEnumerator1" "MYSTERY-BOX" (`self.Value $$`) true false true (`SceneComponent.K2_GetComponentLocation` (`self.door-handle`)) true))

(fn `UserConstructionScript`)