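; Sentry gun NPC that tracks and fires at the player while its linked HitBox overlap has it active.
; Tick turns yaw and pitch parts, then line-traces; a player hit triggers barrel recoil, Bullet spawn, muzzle effects, a moving tracer light and delayed random player offsets.
; Universal_Weapons' bullet-hit event drains Life; at zero the gun collapses into physics pieces, then optionally spawns a replacement inheriting HitBox and Active before destroying itself.
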(event `self.ReceiveBeginPlay`
  (bind _hit_box (`self.Hit box`))
  (bind _returnvalue (`GameplayStatics.GetActorOfClass` "/Game/Core/Player/BluePrints/Player_BP.Player_BP_C"))
  (set `self.Player BP` _returnvalue)
  (bind _returnvalue_2 (`GameplayStatics.GetActorOfClass` "/Game/Core/Weapons/BluePrints/Universal_Weapons.Universal_Weapons_C"))
  (add `/Game/Core/Weapons/BluePrints/Universal_Weapons.Bullet Hit Event` _returnvalue_2 (`|CreateDelegate` :!event `Bullet Hit`))
  (`self.WhileLoop` (`KismetSystemLibrary.IsValid` _hit_box)
    (:`Completed`
      (add `self.OnActorBeginOverlap` _hit_box (`|CreateDelegate` :!event `Overlap`))
      (add `self.OnActorEndOverlap` _hit_box (`|CreateDelegate` :!event `Overlap`)))))

(event `self.ReceiveTick`
  (params (DeltaSeconds :type "Float (single-precision)"))
  (bind _player_bp (`self.Player BP`))
  (bind _arrow (`self.Arrow`))
  (bind _cylinder2 (`self.Cylinder2`))
  (bind _player_bp_2 (`self.Player BP`))
  (bind _muzzle_flash (`self.Muzzle Flash`))
  (bind _pointlight1 (`self.PointLight1`))
  (bind _root_2 (`self.Root 2`))
  (bind _returnvalue (`SceneComponent.K2_GetComponentLocation` _arrow))
  (bind _camera (`/Game/Core/Player/BluePrints/Player_BP.Camera` (`self.Player BP`)))
  (bind _camera_2 (`/Game/Core/Player/BluePrints/Player_BP.Camera` _player_bp))
  (bind (_relativerotation_roll _relativerotation_pitch) (`KismetMathLibrary.BreakRotator` (`SceneComponent.RelativeRotation` _root_2)))
  (bind _returnvalue_location (`KismetMathLibrary.BreakTransform` (`SceneComponent.K2_GetComponentToWorld` _camera)))
  (bind _returnvalue_location_2 (`KismetMathLibrary.BreakTransform` (`SceneComponent.K2_GetComponentToWorld` _camera_2)))
  (bind _returnvalue_2 (+ (`/Game/Core/Player/BluePrints/Player_BP.Local OffSet` _player_bp_2) (`KismetMathLibrary.MakeVector` (`KismetMathLibrary.RandomFloatInRange` 0.0 10.0) (`KismetMathLibrary.RandomFloatInRange` 0.0 10.0) (`KismetMathLibrary.RandomFloatInRange` 0.0 10.0))))
  (bind _returnvalue_3 (+ _returnvalue (* (`SceneComponent.GetForwardVector` _arrow) 5000)))
  (bind (_returnvalue_x _returnvalue_y) (`KismetMathLibrary.BreakVector` (`KismetMathLibrary.Conv_RotatorToVector` (`KismetMathLibrary.FindRelativeLookAtRotation` (`SceneComponent.K2_GetComponentToWorld` (`self.Root`)) (+ _returnvalue_location (`SceneComponent.GetForwardVector` _camera))))))
  (bind (_returnvalue_roll _returnvalue_pitch) (`KismetMathLibrary.BreakRotator` (`KismetMathLibrary.FindRelativeLookAtRotation` (`SceneComponent.K2_GetComponentToWorld` (`self.Root 2`)) (+ _returnvalue_location_2 (`SceneComponent.GetForwardVector` _camera_2) (`KismetMathLibrary.MakeVector` 0.0 0.0 (`KismetMathLibrary.SelectFloat` 0.0 -17.0 (== (`/Game/Core/Player/BluePrints/Player_BP.Half Height` _player_bp) 88.0)))))))
  (`/Engine/EditorBlueprintResources/StandardMacros.Gate` (not (`self.Active?`)) :!label _label
    (:`Exit`
      (`/Engine/EditorBlueprintResources/StandardMacros.Gate` false :!label _label_2
        (:`Exit`
          (`SceneComponent.K2_AddRelativeRotation` (`self.Root`) (`KismetMathLibrary.MakeRotator` 0.0 0.0 (* _returnvalue_y (* (`self.Diffcult Level`) -1))) false false)
          (`SceneComponent.K2_AddRelativeRotation` _root_2 (`KismetMathLibrary.MakeRotator` 0.0 _returnvalue_pitch) false false)
          (`SceneComponent.K2_SetRelativeRotation` _root_2 (`KismetMathLibrary.MakeRotator` 90.0 (* _relativerotation_pitch -1.0)) false false)
          (bind _outhit (`KismetSystemLibrary.LineTraceSingle` :`Start` _returnvalue :`End` _returnvalue_3 :`TraceChannel` "TraceTypeQuery1" :`bTraceComplex` true :`TraceHitColor` (struct :`R` 1.0 :`A` 1.0) :`DrawTime` 1.0))
          (bind (_bblockinghit _binitialoverlap _time _distance _location _impactpoint _normal _impactnormal _physmat _hitactor _hitcomponent _hitbonename _bonename _hititem _elementindex _faceindex _tracestart _traceend) (`GameplayStatics.BreakHitResult` _outhit))
          (bind _returnvalue_4 (== _hitactor (`self.Player BP`)))
          (if _returnvalue_4
            (`|ExecutionSequence`
              (:`then_0`
                (`|ExecutionSequence`
                  (:`then_0`
                    (`SceneComponent.K2_SetRelativeLocation` _cylinder2 (`KismetMathLibrary.VInterpTo` (`SceneComponent.RelativeLocation` _cylinder2) (-1448.086959 -142.572224 3e-06) 0.1 5.0) false false)
                    (`KismetSystemLibrary.Delay` 0.1)
                    (`GameplayStatics.PlaySoundAtLocation` "/Game/Core/NPC/Sentry_Gun/Sounds/Fire/Sentry_Gun_Fire.Sentry_Gun_Fire" (`self.K2_GetActorLocation`) (struct) 1.0 1.0 0.0 null null null null)
                    (`SceneComponent.K2_AddRelativeLocation` (`self.Cylinder2`) (100.0 0.0 0.0) false false)
                    (`|SpawnActorFromClass` "/Game/Core/Weapons/BluePrints/Bullet.Bullet_C" (`SceneComponent.K2_GetComponentToWorld` (`self.Arrow1`)) "AlwaysSpawn" "MultiplyWithRoot" null "NewEnumerator5" null null)
                    (`|ExecutionSequence`
                      (:`then_0`
                        (`SceneComponent.K2_SetRelativeRotation` _muzzle_flash (`KismetMathLibrary.MakeRotator` 0.0 0.0 (`KismetMathLibrary.RandomFloatInRange` -359.0 359.0)) false false)
                        (`SceneComponent.SetRelativeScale3D` _muzzle_flash (`KismetMathLibrary.Conv_DoubleToVector` (`KismetMathLibrary.RandomFloatInRange` 6.0 8.6)))
                        (`SceneComponent.SetVisibility` _muzzle_flash true false)
                        (`SceneComponent.SetVisibility` (`self.Smoke Casing`) true false)
                        (`SceneComponent.SetVisibility` (`self.PointLight`) true false)
                        (`KismetSystemLibrary.Delay` 0.05)
                        (`SceneComponent.SetVisibility` _muzzle_flash false false)
                        (`SceneComponent.SetVisibility` (`self.Smoke Casing`) false false)
                        (`SceneComponent.SetVisibility` (`self.PointLight`) false false))))
                  (:`then_1`
                    (`KismetSystemLibrary.Delay` (/ _time 3.0))
                    (if _returnvalue_4
                      (set `/Game/Core/Player/BluePrints/Player_BP.Local OffSet` _returnvalue_2 _player_bp_2)
                      (set `/Game/Core/Player/BluePrints/Player_BP.Rotation Offset` (/ _returnvalue_2 10) _player_bp_2)))))
              (:`then_1`
                (bind _result (`self.IncrementFloat` (`self.NewVar`) 0.1 :!label _label_3)
                  (:`  `
                    (bind _output_get (set `self.NewVar` _result))
                    (`SceneComponent.K2_SetWorldLocation` (`self.PointLight1`) (`KismetMathLibrary.VLerp` _returnvalue _returnvalue_3 (`self.NewVar`)) false false)
                    (if (>= _output_get 1.0)
                      (set `self.NewVar` 0.0)
                      (`SceneComponent.SetVisibility` _pointlight1 false true)
                      (else
                        (`SceneComponent.SetVisibility` _pointlight1 true true)))))))
            (elif (not (== (`self.NewVar`) 0.0))
              (goto _label_3))))))))

(event `Overlap` :!signature `self.OnActorBeginOverlap`
  (params (OverlappedActor :type "Actor Object Reference") (OtherActor :type "Actor Object Reference"))
  (if (== OtherActor (`self.Player BP`))
    (`/Engine/EditorBlueprintResources/StandardMacros.FlipFlop`
      (:`A`
        (set `self.Active?` true)
        (goto _label :!via `Toggle`))
      (:`B`
        (set `self.Active?` false)
        (goto _label :!via `Toggle`)))))

(event `Bullet Hit`
  (params (`Out Hit` :type "HitResult Structure") (`Hit Delay` :type "Float (double-precision)") (Damage :type Integer))
  (bind _box (`self.Box`))
  (if (== (`.HitActor` (`GameplayStatics.BreakHitResult` `Out Hit`)) self)
    (bind _output_get (set `self.Life` (- (`self.Life`) Damage)))
    (if (<= _output_get 0.0)
      (`/Engine/EditorBlueprintResources/StandardMacros.IsValid` _box
        (:`Is Valid`
          (`ActorComponent.K2_DestroyComponent` _box))
        (:`Is Not Valid`
          _))
      (`PrimitiveComponent.SetSimulatePhysics` (`self.Cube`) true)
      (`PrimitiveComponent.SetSimulatePhysics` (`self.Cube1`) true)
      (`PrimitiveComponent.SetSimulatePhysics` (`self.Cube2`) true)
      (`PrimitiveComponent.SetSimulatePhysics` (`self.Cube3`) true)
      (`PrimitiveComponent.SetSimulatePhysics` (`self.Root`) true)
      (`PrimitiveComponent.SetSimulatePhysics` (`self.Root 2`) true)
      (`PrimitiveComponent.SetSimulatePhysics` (`self.Cylinder1`) true)
      (`PrimitiveComponent.SetSimulatePhysics` (`self.Cube5`) true)
      (`PrimitiveComponent.SetSimulatePhysics` (`self.Cube8`) true)
      (`PrimitiveComponent.SetSimulatePhysics` (`self.Cube7`) true)
      (`PrimitiveComponent.SetSimulatePhysics` (`self.Cylinder2`) true)
      (`PrimitiveComponent.SetSimulatePhysics` (`self.Cylinder5`) true)
      (`PrimitiveComponent.SetSimulatePhysics` (`self.Cylinder3`) true)
      (`PrimitiveComponent.SetSimulatePhysics` (`self.Cube4`) true)
      (`PrimitiveComponent.SetSimulatePhysics` (`self.Cube6`) true)
      (`GameplayStatics.PlaySoundAtLocation` "/Game/Core/NPC/Sentry_Gun/Sounds/Destroyed/Sentry_Destroy.Sentry_Destroy" (`self.K2_GetActorLocation`) (struct) 1.0 1.0 0.0 null null null null)
      (`|ExecutionSequence`
        (:`then_0`
          (goto _label_2 :!via `Close`))
        (:`then_1`
          (`KismetSystemLibrary.Delay` 2.0)
          (if (`self.Respawn?`)
            (set `self.Life` 150.0)
            (bind _returnvalue (`|SpawnActorFromClass` "Sentry_Gun_BP_C" (`self.GetTransform`) "AlwaysSpawn" "MultiplyWithRoot" null null))
            (set `/Game/Core/NPC/Sentry_Gun/Sentry_Gun_BP.Hit box` (`self.Hit box`) _returnvalue)
            (set `/Game/Core/NPC/Sentry_Gun/Sentry_Gun_BP.Active?` (`self.Active?`) _returnvalue))
          (`self.K2_DestroyActor`))))))

(fn `UserConstructionScript`)